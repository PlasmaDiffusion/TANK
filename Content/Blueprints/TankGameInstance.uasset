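; Game instance for a tank game that prepares the list of dungeon rooms to load when it initializes.
; Init builds a pool of normal room names from an "NR" prefix plus index, then calls PickLevels.
; PickLevels fills every dungeon room slot with the first pool entry; a random-integer node is present but unused, so selection is not randomized.
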(event `self.ReceiveInit`
  ;[1 1 1] NormalRooms
  (for _index (range 2)
    (`KismetArrayLibrary.Array_Set` (`self.normalRoomsToPickFrom`) _index (`KismetSystemLibrary.MakeLiteralName` (`KismetStringLibrary.Conv_StringToName` (`KismetStringLibrary.Concat_StrStr` "NR" (`KismetStringLibrary.Conv_IntToString` _index)))) true))
  (`self.PickLevels`))

(fn `PickLevels`
  (for _index (range 49)
    (`KismetArrayLibrary.Array_Set` (`self.dungeonRoomsToLoad`) _index (`|GetArrayItem` (`self.normalRoomsToPickFrom`)) true)))