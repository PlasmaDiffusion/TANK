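; BP_SplineEnemy is an enemy that travels continuously along the spline of a referenced spline actor.
; Each Tick advances a normalized SplineLerp by world delta time times TankLerpSpeed, scales it by spline length, and sets the world location at that distance.
; LoopLerp resets the value to zero once it exceeds one, so the path repeats from the start.
; Movement sets location only, without sweep or rotation.
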(event `self.ReceiveBeginPlay`
  (`parent.ReceiveBeginPlay`))

(event `self.ReceiveTick`
  (params (DeltaSeconds :type "Float (single-precision)"))
  (`parent.ReceiveTick` DeltaSeconds)
  (`self.LoopLerp`)
  (set `self.splineLerp` (+ (`self.splineLerp`) (* (`GameplayStatics.GetWorldDeltaSeconds`) (`self.tankLerpSpeed`))))
  (`self.K2_SetActorLocation` (`SplineComponent.GetLocationAtDistanceAlongSpline` (`/Game/Blueprints/Enemies/BP_SplinePath.Spline` (`self.splineActorReference`)) (* (`SplineComponent.GetSplineLength` (`/Game/Blueprints/Enemies/BP_SplinePath.Spline` (`self.splineActorReference`))) (`self.splineLerp`)) "World")))

(fn `LoopLerp`
  (if (> (`self.splineLerp`) 1.0)
    (set `self.splineLerp` 0.0))
  (return))

(fn `UserConstructionScript`
  (`parent.UserConstructionScript`))