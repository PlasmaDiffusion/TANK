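; Room door for the twin-stick game, with two sliding panels, bars and a lock, gated by a door Type enum.
; Box overlaps slide the panels open for projectiles on eligible types, or let the player pawn unlock key and boss-key doors.
; Unlocking removes the lock and lowers the bars; both motions are timeline-driven lerps.
; Helper functions hide the lock, restyle it for a boss, apply wall material, or lower bars by type.
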(event `self.ReceiveBeginPlay`)

(event `SlideDoors`
  (bind (_direction _newtrack_0) (`Timeline|Timeline_SlideDoors` :!via `PlayFromStart`)
    (:`Update`
      (`SceneComponent.K2_SetRelativeLocation` (`self.DoorL`) (`KismetMathLibrary.VLerp` (100.0 0.0 0.0) (0.0 0.0 0.0) _newtrack_0) false false)
      (`SceneComponent.K2_SetRelativeLocation` (`self.DoorR`) (`KismetMathLibrary.VLerp` (100.0 0.0 0.0) (200.0 0.0 0.0) _newtrack_0) false false))))

(event `self.DoorL.OnComponentHit`
  (params (HitComponent :type "PrimitiveComponent Object Reference") (OtherActor :type "Actor Object Reference") (OtherComp :type "PrimitiveComponent Object Reference") (NormalImpulse :type "Vector Structure") (Hit :type "HitResult Structure (by ref)")))

(event `self.DoorR.OnComponentHit`
  (params (HitComponent :type "PrimitiveComponent Object Reference") (OtherActor :type "Actor Object Reference") (OtherComp :type "PrimitiveComponent Object Reference") (NormalImpulse :type "Vector Structure") (Hit :type "HitResult Structure (by ref)")))

(event `self.Box.OnComponentBeginOverlap`
  (params (OverlappedComponent :type "PrimitiveComponent Object Reference") (OtherActor :type "Actor Object Reference") (OtherComp :type "PrimitiveComponent Object Reference") (OtherBodyIndex :type Integer) (bFromSweep :type Boolean) (SweepResult :type "HitResult Structure (by ref)"))
  (bind _castsuccess (`self.HitToOpen` OtherActor))
  (if (not _castsuccess)
    (bind _asbp_twin_stick_pawn (cast `/Game/Blueprints/BP_TwinStickPawn` OtherActor))
    (`self.UnlockDoor` _asbp_twin_stick_pawn)))

(event `LowerBarEvent`
  (bind _x (.x (`SceneComponent.RelativeLocation` (`self.Bars`))))
  (bind _y (.y (`SceneComponent.RelativeLocation` (`self.Bars`))))
  (if (`|EnumEquality` (`self.type`) "NewEnumerator2")
    (set `self.type` "NewEnumerator1")
    (bind (_direction _newtrack_0) (`Timeline|Timeline_Bars` :!via `PlayFromStart` :!label _label)
      (:`Update`
        (`SceneComponent.K2_SetRelativeLocation` (`self.Bars`) (`KismetMathLibrary.VLerp` (`KismetMathLibrary.MakeVector` _x _y) (`KismetMathLibrary.MakeVector` _x _y -150.0) _newtrack_0) false false)))
    (else
      (goto _label :!via `PlayFromStart`))))

(fn `BecomeWall`
  (`PrimitiveComponent.SetMaterial` (`self.DoorR`) 0 "/Game/Materials/RoomLayout/lambert1.lambert1")
  (`PrimitiveComponent.SetMaterial` (`self.DoorL`) 0 "/Game/Materials/RoomLayout/lambert1.lambert1"))

(fn `HideLock`
  (`SceneComponent.SetVisibility` (`self.Lock`) false false))

(fn `HitToOpen`
  (params (Object :type "Object Object Reference"))
  (returns (castSuccess :type Boolean))
  (cast `/Game/Blueprints/BP_TwinStickProjectile` Object)
  (if (and (`|EnumInequality` (`self.type`) "NewEnumerator0") (`|EnumInequality` (`self.type`) "NewEnumerator3") (`|EnumInequality` (`self.type`) "NewEnumerator4") (`|EnumInequality` (`self.type`) "NewEnumerator2"))
    (`self.SlideDoors`)
    (return true)
    (else
      (return false))))

(fn `LowerBars`
  (if (`|EnumEquality` (`self.type`) "NewEnumerator5")
    (`self.LowerBarEvent`)))

(fn `TurnIntoBossLock`
  (bind _lock (`self.Lock`))
  (`StaticMeshComponent.SetStaticMesh` _lock "/Game/Geometry/RoomLayout/Walls_Door_Keys_Turret_Boss_Lock.Walls_Door_Keys_Turret_Boss_Lock")
  (`PrimitiveComponent.SetMaterial` _lock 0 "/Game/Materials/RoomLayout/blinn7.blinn7"))

(fn `UnlockDoor`
  (params (playerRef :type "/Game/Blueprints/BP_TwinStickPawn Object Reference"))
  (bind _keys (`/Game/Blueprints/BP_TwinStickPawn.keys` playerRef))
  (if (`|EnumEquality` (`self.type`) "NewEnumerator3")
    (if (> _keys 0)
      (`/Engine/EditorBlueprintResources/StandardMacros.DecrementInt` _keys
        (:`  `
          (set `self.type` "NewEnumerator1")
          (`ActorComponent.K2_DestroyComponent` (`self.Lock`))
          (`self.LowerBarEvent`))))
    (elif (`|EnumEquality` (`self.type`) "NewEnumerator4")
      (if (`/Game/Blueprints/TankGameInstance.bossKey` (`/Game/Blueprints/BP_TwinStickPawn.GI` playerRef))
        (set `self.type` "NewEnumerator1")
        (`ActorComponent.K2_DestroyComponent` (`self.Lock`))
        (`self.LowerBarEvent`)))))

(fn `UserConstructionScript`)